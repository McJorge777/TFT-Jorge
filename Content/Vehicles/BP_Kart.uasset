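; Physics-driven player kart that sets up vehicle input and a HUD, with timed speed boosts and a track-spline direction check.
; Each tick, four wheel traces push the box up as spring suspension and apply forward force.
; Ground-gated throttle eases in and decays, scaling drive force, steering torque, center-of-mass shift and wheel spin.
; Stop request and completion events toggle a stop indicator, suggesting bus-style passenger stops.
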(event Input|EnhancedActionEvents|EnhancedInputActionIA_Acelerate
  (params (ActionValue :type Float%20%28double-precision%29) (ElapsedSeconds :type Float%20%28double-precision%29) (TriggeredSeconds :type Float%20%28double-precision%29) (InputAction :type Input%20Action%20Object%20Reference :default "/Game/Inputs/IA_Acelerate.IA_Acelerate"))
  ;[0.15 0.15 0.15 0.5] Aceleracion
  (Variables|Default|SetAccelerationInput (Math|Interpolation|FInterpTo (Variables|Default|GetAccelerationInput) (Math|Float|SelectFloat ActionValue 0.0 (CallFunction|IsonGround)) (Utilities|Time|GetWorldDeltaSeconds) 0.5)))

(event Input|EnhancedActionEvents|EnhancedInputActionIA_Steer
  (params (ActionValue :type Float%20%28double-precision%29) (ElapsedSeconds :type Float%20%28double-precision%29) (TriggeredSeconds :type Float%20%28double-precision%29) (InputAction :type Input%20Action%20Object%20Reference :default "/Game/Inputs/IA_Steer.IA_Steer"))
  ;[0.15 0.15 0.15 0.5] giro de ruedas
  (Class|PrimitiveComponent|AddTorqueinRadians (Variables|Default|GetBox) (Math|Vector|MakeVector 0.0 0.0 (* ActionValue 1e+08 (Variables|Default|GetAccelerationInput))) "None" false)
  (Transformation|SetRelativeRotation (Variables|Default|GetBL_Wheel) (Math|Rotator|MakeRotator 0.0 0.0 (Math|Interpolation|FInterpTo ActionValue (.yaw (Variables|/Script/Engine.SceneComponent|GetRelativeRotation (Variables|Default|GetBL_Wheel))) (Utilities|Time|GetWorldDeltaSeconds) 3.0)) false false))

(event EventBeginPlay
  (Input|AddMappingContext (PlayerController|LocalPlayerSubsystems|GetEnhancedInputLocalPlayerSubsystem (Game|GetPlayerController 0)) "/Game/Inputs/IMC_Vehicle.IMC_Vehicle" 0 "(bIgnoreAllPressedKeysUntilRelease=True,bForceImmediately=False,bNotifyUserSettings=False)")
  (bind _returnvalue (Actor|GetActorOfClass "/Game/Vehicles/BP_TrackSpline.BP_TrackSpline_C"))
  (Variables|Default|SetTrack _returnvalue)
  (bind _returnvalue_2 (UserInterface|CreateWidget "/Game/UI/WBP_HUD.WBP_HUD_C"))
  (bind _output_get (Variables|Default|SetMiHUD _returnvalue_2))
  (UserInterface|Viewport|AddtoViewport _output_get 0))

(event EventCompletarParada
  (if (Variables|Default|GetParadaSolicitada)
    (Variables|Default|SetParadaSolicitada false)
    (Default|ActualizarTestigoParada (Variables|Default|GetTarget) false)
    (Utilities|FlowControl|Delay 2.0)
    (Development|PrintString "Puertas cerradas")))

(event EventTick
  (params (DeltaSeconds :type Float%20%28single-precision%29))
  (CallFunction|SuspensionCast (Variables|Default|GetFL_Wheel))
  (CallFunction|SuspensionCast (Variables|Default|GetFR_Wheel))
  (CallFunction|SuspensionCast (Variables|Default|GetBR_Wheel))
  (CallFunction|SuspensionCast (Variables|Default|GetBL_Wheel))
  (CallFunction|CalculateAcceleration))

(event EventSolicitarParada
  (if (not (Variables|Default|GetParadaSolicitada))
    (Variables|Default|SetParadaSolicitada true)
    (Audio|PlaySound2D "/Engine/EditorSounds/GamePreview/EndPlayInEditor.EndPlayInEditor" 1.0 1.0 0.0 0 0)
    (Default|ActualizarTestigoParada (Variables|Default|GetTarget) true)))

(fn ConstructionScript)

(fn SuspensionCast
  (params (WheelComp :type Scene%20Component%20Object%20Reference))
  (bind _returnvalue (Transformation|GetWorldLocation WheelComp))
  (bind _returnvalue_2 (Components|GetChildComponent WheelComp 0))
  (bind _outhit (Collision|LineTraceByChannel _returnvalue (+ _returnvalue (* (Math|Vector|GetUpVector WheelComp) -6e+01)) "TraceTypeQuery1" false 0 "ForOneFrame"))
  (if (.bBlockingHit (Collision|BreakHitResult _outhit))
    (Class|PrimitiveComponent|AddForceatLocation (Variables|Default|GetBox) (* (- 1.0 (Math|Float|NormalizetoRange (.Distance (Collision|BreakHitResult _outhit)) 0.0 6e+01)) (Math|Vector|GetUnitDirection(Vector) (.TraceEnd (Collision|BreakHitResult _outhit)) (.TraceStart (Collision|BreakHitResult _outhit))) 9e+05) (Transformation|GetWorldLocation WheelComp) "None")
    (CallFunction|AccelerateKart WheelComp)
    (Transformation|SetRelativeLocation _returnvalue_2 (Math|Vector|MakeVector 0.0 0.0 (Math|Interpolation|FInterpTo (.z (Variables|/Script/Engine.SceneComponent|GetRelativeLocation _returnvalue_2)) (+ (* (.Distance (Collision|BreakHitResult _outhit)) -1.0) 5e+01) (Utilities|Time|GetWorldDeltaSeconds) 0.0)) false false)
    (else
      (CallFunction|AccelerateKart WheelComp))))

(fn CalculateAcceleration
  (bind _output_get (Variables|Default|SetAcceleration (* (Math|Float|Lerp 0.0 1.5e+04 (Variables|Default|GetAccelerationInput)) (Variables|Default|GetAccelerationInput))))
  (Variables|Default|SetAccelerationInput (Math|Interpolation|FInterpTo (Variables|Default|GetAccelerationInput) 0.0 (Utilities|Time|GetWorldDeltaSeconds) 0.3))
  (Transformation|AddLocalRotation (Variables|Default|GetWheel_BL) (Math|Rotator|MakeRotator 0.0 0.0 (/ _output_get -1e+03)) false false))

(fn AccelerateKart
  (params (WheelComp :type Scene%20Component%20Object%20Reference))
  (bind _box (Variables|Default|GetBox))
  (Class|PrimitiveComponent|AddForceatLocation (Variables|Default|GetBox) (* (Math|Vector|GetForwardVector _box) 1.5e+03 (Variables|Default|GetAccelerationInput) (Physics|GetMass _box) (Variables|Default|GetSpeedModifier)) (Transformation|GetWorldLocation WheelComp) "None")
  (Class|PrimitiveComponent|SetCenterOfMass (Variables|Default|GetBox) (* "50.000000,0.000000,0.000000" (Variables|Default|GetAccelerationInput)) "None"))

(fn IsonGround
  (bind _returnvalue (Transformation|GetActorLocation))
  (bind _returnvalue_2 (Collision|MultiLineTraceByChannel _returnvalue (- _returnvalue "0.000000,0.000000,55.000000") "TraceTypeQuery1" false 0 "None"))
  (return _returnvalue_2))

(fn GetTrackProgress
  (return (> (Math|Vector|DotProduct (Spline|FindDirectionClosesttoWorldLocation (Variables|/Game/Vehicles/BP_TrackSpline.BP_TrackSpline_C|GetSpline (Variables|Default|GetTrack)) (Transformation|GetActorLocation) "World") (Math|Vector|Normalize (Transformation|GetVelocity))) 0.0)))

(fn BoostKart
  (params (SpeedModifier :type Float%20%28single-precision%29) (Time :type Float%20%28single-precision%29))
  (Variables|Default|SetSpeedModifier SpeedModifier)
  (Utilities|Time|SetTimerbyFunctionName 0 "ResetSpeed" Time))

(fn ResetSpeed
  (Variables|Default|SetSpeedModifier 1.0))