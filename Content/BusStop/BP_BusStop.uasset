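; BP_BusStop is a bus stop that randomly requests a stop from an approaching vehicle and detects when it has pulled in.
; Overlapping TriggerAviso rolls a weighted chance to activate the stop and messages the overlapping actor.
; While active, overlapping ZonaDetencion starts a looping timer that polls the vehicle's speed.
; Once nearly stationary, the timer clears, the stop deactivates and the vehicle receives a completion message, without checking it remains inside.
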(event OnComponentBeginOverlap(TriggerAviso)
  (params (OverlappedComponent :type Primitive%20Component%20Object%20Reference) (OtherActor :type Actor%20Object%20Reference) (OtherComp :type Primitive%20Component%20Object%20Reference) (OtherBodyIndex :type Integer) (bFromSweep :type Boolean) (SweepResult :type Hit%20Result%20Structure%20%28by%20ref%29))
  (if (Math|Random|RandomBoolwithWeight (Variables|Default|GetProbabilidadParada))
    (Variables|Default|SetParadaActiva true)
    (Class|BPIStopSystem|SolicitarParada(Message) OtherActor)))

(event OnComponentBeginOverlap(ZonaDetencion)
  (params (OverlappedComponent :type Primitive%20Component%20Object%20Reference) (OtherActor :type Actor%20Object%20Reference) (OtherComp :type Primitive%20Component%20Object%20Reference) (OtherBodyIndex :type Integer) (bFromSweep :type Boolean) (SweepResult :type Hit%20Result%20Structure%20%28by%20ref%29))
  (if (Variables|Default|GetParadaActiva)
    (Variables|Default|SetVehiculoEnZona OtherActor)
    (bind _returnvalue (Utilities|Time|SetTimerbyEvent (delegate Custom|CheckFrenado) 0.2 true))
    (Variables|Default|SetTimerComprobarVelocidad _returnvalue)))

(event Custom|CheckFrenado
  (if (< (Math|Vector|VectorLength (Transformation|GetVelocity (Variables|Default|GetVehiculoEnZona))) 5.0)
    (Utilities|Time|ClearandInvalidateTimerbyHandle (Variables|Default|GetTimerComprobarVelocidad))
    (Variables|Default|SetParadaActiva false)
    (Class|BPIStopSystem|CompletarParada(Message) (Variables|Default|GetVehiculoEnZona))))

(event EventBeginPlay)

(event Collision|EventActorBeginOverlap
  (params (OtherActor :type Actor%20Object%20Reference)))

(event EventTick
  (params (DeltaSeconds :type Float%20%28single-precision%29)))

(fn ConstructionScript)